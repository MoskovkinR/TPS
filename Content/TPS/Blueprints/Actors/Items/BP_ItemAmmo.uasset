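; Ammo pickup item that refills the current weapon of the actor that collects it.
; Both sphere overlap and the Interact event call a shared function that reads CurrentWeapon from the actor's TPSWeaponComponent.
; If that weapon is valid, it receives a configurable number of clips and no loose bullets.
; The pickup destroys itself only when AddAmmo reports success, so otherwise it stays in the world.
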(event OnComponentBeginOverlap(Sphere)
  (params (OverlappedComponent :type Primitive%20Component%20Object%20Reference) (OtherActor :type Actor%20Object%20Reference) (OtherComp :type Primitive%20Component%20Object%20Reference) (OtherBodyIndex :type Integer) (bFromSweep :type Boolean) (SweepResult :type Hit%20Result%20Structure%20%28by%20ref%29))
  (CallFunction|InteractWhithAmmo OtherActor))

(event EventBeginPlay
  (|CallParentFunction) ; This node is disabled and will not be called.\nDrag off pins to build functionality.
)

(event EventInteract
  (params (Actor :type Actor%20Object%20Reference))
  (CallFunction|InteractWhithAmmo Actor))

(fn ConstructionScript
  (|CallParentFunction))

(fn InteractWhithAmmo
  (params (ActorTo :type Actor%20Object%20Reference))
  (bind _returnvalue (Actor|GetComponentbyClass ActorTo "/Script/TPS.TPSWeaponComponent"))
  (bind _currentweapon (Variables|/Script/TPS.TPSWeaponComponent|GetCurrentWeapon _returnvalue))
  (Utilities|IsValid _currentweapon
    (:Is%20Valid
      (bind _returnvalue_2 (Class|TPSBaseWeaponGame|AddAmmo _currentweapon (Utilities|Struct|MakeAmmoData 0 (Variables|Default|GetAddAmmoClips))))
      (if _returnvalue_2
        (Actor|DestroyActor)))))