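; TPS player character Blueprint that adds the HUD, inventory screen and world interaction for the player.
; BeginPlay creates the W_HUD widget and stores a reference to it.
; The I key creates a new inventory widget on each press and fills its grid from the BACInventorySystem component.
; The E key uses a short-range aim point check and sends InteractMessage to hit actors implementing the BP_Interactable interface.
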(event EventBeginPlay
  (bind _returnvalue (UserInterface|CreateWidget "/Game/TPS/Widgets/HUD/W_HUD.W_HUD_C"))
  (Variables|Default|SetHUD_Ref _returnvalue)
  (UserInterface|Viewport|AddtoViewport (Variables|Default|GetHUD_Ref) 0))

(event Input|KeyboardEvents|I
  (params (Key :type Key%20Structure :default "None"))
  (:Pressed
    (bind _returnvalue (UserInterface|CreateWidget "/Game/TPS/Widgets/Inventory/W_Inventory.W_Inventory_C" (Game|GetPlayerController 0)))
    (UserInterface|Viewport|AddtoViewport _returnvalue 0)
    (Default|DisplayInventory (Variables|/Game/TPS/Widgets/Inventory/W_Inventory.W_Inventory_C|GetWBP_InventoryGrid _returnvalue) (Variables|Default|GetBAC_InventorySystem))))

(event Input|KeyboardEvents|E
  (params (Key :type Key%20Structure :default "None"))
  (bind _hitresult (Class|TPSBaseCharacter|GetAimPoint 5e+02))
  (bind (_bblockinghit _binitialoverlap _time _distance _location _impactpoint _normal _impactnormal _physmat _hitactor) (Collision|BreakHitResult _hitresult))
  (:Pressed
    (if _bblockinghit
      (if (Utilities|DoesObjectImplementInterface _hitactor "/Game/TPS/Blueprints/Interface/BP_Interactable.BP_Interactable_C")
        (Class|BPInteractable|Interact(Message) _hitactor self)))))

(fn ConstructionScript)